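; Player-controlled tank Blueprint with an orbiting aim camera and a fire action.
; Construction assigns turret and barrel meshes and materials, and BeginPlay passes both components to SetTurretReference and SetBarrelReference.
; Aim axes yaw the azimuth gimbal and pitch the spring arm separately, while the Fire input calls Fire.
; Tick feeds the tank's speed into the particle system's InitialVelocity Z, scaling the effect with movement.
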(event `self.ReceiveBeginPlay`
  (`self.SetBarrelReference` (`self.Barrel`))
  (`self.SetTurretReference` (`self.Turret`)))

(event `self.ReceiveTick`
  (params (DeltaSeconds :type "Float (single-precision)"))
  (`ParticleSystemComponent.SetVectorParameter` (`self.ParticleSystem`) "InitialVelocity" (`KismetMathLibrary.MakeVector` 0.0 0.0 (`KismetMathLibrary.VSize` (`self.GetVelocity`)))))

(event `InputAxis|AimAzimuth`
  (params (AxisValue :type "Float (single-precision)"))
  ;[1 1 1] Camera Stuff
  (`SceneComponent.K2_AddLocalRotation` (`self.Azimuth Gimbal`) (`KismetMathLibrary.MakeRotator` 0.0 0.0 AxisValue) false false))

(event `InputAxis|AimElevation`
  (params (AxisValue :type "Float (single-precision)"))
  ;[1 1 1] Camera Stuff
  (`SceneComponent.K2_AddLocalRotation` (`self.SpringArm`) (`KismetMathLibrary.MakeRotator` 0.0 AxisValue) false false))

(event `InputAction|Fire`
  (params (Key :type "Key Structure"))
  ;[1 1 1] Tank Input
  (:`Pressed`
    (`self.Fire`)))

(fn `UserConstructionScript`
  (bind _barrel (`self.Barrel`))
  (bind _turret (`self.Turret`))
  (`StaticMeshComponent.SetStaticMesh` _turret "/Game/Tank/tank_fbx_Turret.tank_fbx_Turret")
  (`PrimitiveComponent.SetMaterial` _turret 0 "/Game/Tank/M_TankBase.M_TankBase")
  (`StaticMeshComponent.SetStaticMesh` _barrel "/Game/Tank/tank_fbx_Barrel.tank_fbx_Barrel")
  (`PrimitiveComponent.SetMaterial` _barrel 0 "/Game/Tank/M_TankBarrel.M_TankBarrel"))